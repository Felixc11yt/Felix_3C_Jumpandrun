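; Player character with Enhanced Input movement, look and jump, plus looping run sounds throttled by a Delay on Tick.
; Any damage triggers a hide, fade and teleport to the respawn transform, taken from PlayerStart or the latest checkpoint.
; A CanMove counter blocks look and jump during respawn.
; Interact messages the registered interactable best aligned with the actor's forward vector by dot product, then removes it from the list.
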(event `self.ReceiveTick`
  (params (DeltaSeconds :type "Float (single-precision)"))
  (bind _charactermovement (`self.CharacterMovement`))
  (bind _output_get (set `self.Speed` (`KismetMathLibrary.VSizeXY` (`MovementComponent.Velocity` _charactermovement))))
  (if (and (> _output_get 10.0) (`NavMovementInterface.IsMovingOnGround` _charactermovement))
    (`KismetSystemLibrary.Delay` 0.45)
    (`GameplayStatics.PlaySound2D` "/Game/Audio/MetaSounds/MS_Run.MS_Run" 1.0 1.0 0.0 null null false)))

(event `self.ReceiveBeginPlay`
  (bind _returnvalue (`GameplayStatics.GetActorOfClass` "/Script/Engine.PlayerStart"))
  (set `self.Respawn Transform` (`self.GetTransform` _returnvalue))
  (set `self.GravityScaleRef` (`CharacterMovementComponent.GravityScale` (`self.CharacterMovement`))))

(event `EnhancedInput|/Game/Inputs/IA_Look`
  (params (ActionValue :type "Vector2D Structure") (ElapsedSeconds :type "Float (double-precision)") (TriggeredSeconds :type "Float (double-precision)") (InputAction :type "InputAction Object Reference" :default "/Game/Inputs/IA_Look.IA_Look"))
  (bind (_x _y) (`KismetMathLibrary.BreakVector2D` ActionValue))
  (:`Triggered`
    (`self.CanMoveState`
      (:`CanMove`
        (`self.AddControllerYawInput` _x)
        (`self.AddControllerPitchInput` _y)))))

(event `EnhancedInput|/Game/Inputs/IA_Move`
  (params (ActionValue :type "Vector2D Structure") (ElapsedSeconds :type "Float (double-precision)") (TriggeredSeconds :type "Float (double-precision)") (InputAction :type "InputAction Object Reference" :default "/Game/Inputs/IA_Move.IA_Move"))
  (bind (_x _y) (`KismetMathLibrary.BreakVector2D` ActionValue))
  (bind (_returnvalue_roll _returnvalue_pitch _returnvalue_yaw) (`KismetMathLibrary.BreakRotator` (`self.GetControlRotation`)))
  (bind (_returnvalue_roll_2 _returnvalue_pitch_2 _returnvalue_yaw_2) (`KismetMathLibrary.BreakRotator` (`self.GetControlRotation`)))
  (:`Triggered`
    (`self.AddMovementInput` (`KismetMathLibrary.GetRightVector` (`KismetMathLibrary.MakeRotator` 0.0 0.0 _returnvalue_yaw)) _x)
    (`self.AddMovementInput` (`KismetMathLibrary.GetForwardVector` (`KismetMathLibrary.MakeRotator` 0.0 0.0 _returnvalue_yaw_2)) _y)))

(event `EnhancedInput|/Game/Inputs/IA_Jump`
  (params (ActionValue :type Boolean) (ElapsedSeconds :type "Float (double-precision)") (TriggeredSeconds :type "Float (double-precision)") (InputAction :type "InputAction Object Reference" :default "/Game/Inputs/IA_Jump.IA_Jump"))
  (:`Started`
    (if (== (`self.CanMove`) 0)
      (`self.Jump`)))
  (:`Completed`
    (`self.StopJumping`)))

(event `self.ReceiveAnyDamage`
  (params (Damage :type "Float (single-precision)") (DamageType :type "DamageType Object Reference") (InstigatedBy :type "Controller Object Reference") (DamageCauser :type "Actor Object Reference"))
  (bind _charactermovement (`self.CharacterMovement`))
  (bind _rotation (.rotation (`self.Respawn Transform`)))
  (`/Engine/EditorBlueprintResources/StandardMacros.IncrementInt` (`self.CanMove`)
    (:`  `
      (`self.SetActorHiddenInGame` true)
      (`KismetSystemLibrary.DelayUntilNextTick`)
      (set `CharacterMovementComponent.GravityScale` 0.0 _charactermovement)
      (set `MovementComponent.Velocity` (0.0 0.0 0.0) _charactermovement)
      (`KismetSystemLibrary.Delay` 0.1)
      (`PlayerCameraManager.StartCameraFade` :`self` (`GameplayStatics.GetPlayerCameraManager` 0) :`ToAlpha` 1.0 :`Duration` 1.0 :`bShouldFadeAudio` true :`bHoldWhenFinished` true)
      (`KismetSystemLibrary.Delay` 1.2)
      (`self.K2_SetActorLocationAndRotation` (.location (`self.Respawn Transform`)) _rotation false true)
      (`Controller.SetControlRotation` (`GameplayStatics.GetPlayerController` 0) _rotation)
      (set `CharacterMovementComponent.GravityScale` (`self.GravityScaleRef`) (`self.CharacterMovement`))
      (`self.SetActorHiddenInGame` false)
      (`/Engine/EditorBlueprintResources/StandardMacros.DecrementInt` (`self.CanMove`)
        (:`  `
          (`PlayerCameraManager.StartCameraFade` :`self` (`GameplayStatics.GetPlayerCameraManager` 0) :`FromAlpha` 1.0 :`Duration` 1.0 :`bShouldFadeAudio` true))))))

(event `/Game/Blueprints/Interfaces/BPI_Player.CheckpointReached`
  (params (CheckpointRef :type "/Game/Blueprints/Stuff/BP_CheckPoint Object Reference"))
  (bind _currentcheckpoint (`self.CurrentCheckpoint`)
    (:`then`
      (if (!= _currentcheckpoint CheckpointRef)
        (`/Game/Blueprints/Stuff/BP_CheckPoint.DeactivateCheckpoint` (`self.CurrentCheckpoint`))
        (bind _output_get (set `self.CurrentCheckpoint` CheckpointRef :!label _label))
        (set `self.Respawn Transform` (`SceneComponent.K2_GetComponentToWorld` (`/Game/Blueprints/Stuff/BP_CheckPoint.Arrow` _output_get)))))
    (:`else`
      (goto _label))))

(event `EnhancedInput|/Game/Inputs/IA_Interact`
  (params (ActionValue :type Boolean) (ElapsedSeconds :type "Float (double-precision)") (TriggeredSeconds :type "Float (double-precision)") (InputAction :type "InputAction Object Reference" :default "/Game/Inputs/IA_Interact.IA_Interact"))
  (bind _interactable (`self.GetLookAtInteractable`))
  (:`Started`
    (if (`KismetSystemLibrary.IsValid` _interactable)
      (message `/Game/Blueprints/Interfaces/BPI_Interact.Interact` _interactable self)
      (`KismetArrayLibrary.Array_RemoveItem` (`self.Interactables`) _interactable))))

(event `/Game/Blueprints/Interfaces/BPI_Player.UpdateInteractables`
  (params (Interactable :type "Actor Object Reference") (Add :type Boolean))
  (if Add
    (`KismetArrayLibrary.Array_AddUnique` (`self.Interactables`) Interactable)
    (else
      (`KismetArrayLibrary.Array_RemoveItem` (`self.Interactables`)))))

(fn `GetLookAtInteractable`
  (returns (Interactable :type "Actor Object Reference"))
  (locals (LookAtValue :type "Float (double-precision)" :default -1.1) (LookAtInteractable :type "Actor Object Reference"))
  (for _array_element (`self.Interactables`)
    (if (`KismetSystemLibrary.IsValid` _array_element)
      (bind _returnvalue (`KismetMathLibrary.Dot_VectorVector` (`KismetMathLibrary.Normal` (- (`self.K2_GetActorLocation` _array_element) (- (`self.K2_GetActorLocation`) (`KismetMathLibrary.MakeVector` 0.0 0.0 (`CapsuleComponent.CapsuleHalfHeight` (`self.CapsuleComponent`)))))) (`self.GetActorForwardVector`)))
      (if (> _returnvalue (`local.LookAtValue`))
        (set `local.LookAtInteractable` _array_element)
        (set `local.LookAtValue` _returnvalue))))
  (return (`local.LookAtInteractable`)))

(fn `UserConstructionScript`)