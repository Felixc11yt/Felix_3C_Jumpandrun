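; BP_CheckPoint is a checkpoint trigger that the player activates by overlapping its box.
; Two meshes, Cube and Cube1, serve as inactive and active visuals, with Cube1 hidden at start.
; On overlap by BP_Player it swaps their visibility and passes itself to the player through CheckpointReachedMessage.
; DeactivateCheckpoint reverses the swap to restore the inactive look.
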(event `self.ReceiveBeginPlay`
  (`SceneComponent.SetHiddenInGame` (`self.Cube1`) true false))

(event `self.Box.OnComponentBeginOverlap`
  (params (OverlappedComponent :type "PrimitiveComponent Object Reference") (OtherActor :type "Actor Object Reference") (OtherComp :type "PrimitiveComponent Object Reference") (OtherBodyIndex :type Integer) (bFromSweep :type Boolean) (SweepResult :type "HitResult Structure (by ref)"))
  (if (== (`GameplayStatics.GetObjectClass` OtherActor) "/Game/Blueprints/BP_Player.BP_Player_C")
    (`SceneComponent.SetHiddenInGame` (`self.Cube`) true false)
    (`SceneComponent.SetHiddenInGame` (`self.Cube1`) false false)
    (message `/Game/Blueprints/Interfaces/BPI_Player.CheckpointReached` OtherActor self)))

(event `DeactivateCheckpoint`
  (`SceneComponent.SetHiddenInGame` (`self.Cube`) false false)
  (`SceneComponent.SetHiddenInGame` (`self.Cube1`) true false))

(fn `UserConstructionScript`)